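; Enemy ship Blueprint for the space shooter that fires bullets from two fire points.
; Tick moves it along its movement vector at its speed and calls Fire whenever the shoot timer exceeds the delay.
; FireBurst spawns an enemy bullet at each fire point and sets the delay to a short interval; its caller is not in this graph.
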(event `self.ReceiveTick`
  (params (DeltaSeconds :type "Float (single-precision)"))
  (`self.K2_SetActorLocation` (+ (`self.K2_GetActorLocation`) (* (* DeltaSeconds (`self.Speed`)) (`self.MovementVector`))))
  (set `self.ShootCurrentTime` (+ (`self.ShootCurrentTime`) DeltaSeconds))
  (if (> (`self.ShootCurrentTime`) (`self.DelayShoot`))
    (`self.Fire`)
    (set `self.ShootCurrentTime` 0.0)))

(fn `FireBurst`
  (`|SpawnActorFromClass` "/Game/00_Space_Shooter/Enemies/EnemyBullet.EnemyBullet_C" (`SceneComponent.K2_GetComponentToWorld` (`self.FirePoint1`)) "Undefined" "MultiplyWithRoot" null null)
  (set `self.DelayShoot` 0.2)
  (`|SpawnActorFromClass` "/Game/00_Space_Shooter/Enemies/EnemyBullet.EnemyBullet_C" (`SceneComponent.K2_GetComponentToWorld` (`self.FirePoint2`)) "Undefined" "MultiplyWithRoot" null null))

(fn `UserConstructionScript`
  (`parent.UserConstructionScript`))